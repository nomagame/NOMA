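; VR context Blueprint for the Ximmerse SDK that starts the device plugin and handles recentering input.
; On BeginPlay it sets the play-area wall renderer, then initializes XDevicePlugin with itself after a short delay.
; Pressed flags detect a two-Home-button chord that recenters the tracker, while a single press recenters all controllers.
; Both paths reset headset orientation, and keys T and R trigger them from the keyboard.
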(event `self.ReceiveBeginPlay`
  (bind _xdeviceplugin (`self.XDevicePlugin`))
  (`XDevicePluginComponent.SetPlayAreaRenderer` _xdeviceplugin (`self.PlayAreaRenderer-Wall`))
  (`KismetSystemLibrary.Delay` 0.2)
  (`XDevicePluginComponent.Init` _xdeviceplugin self))

(event `Key|XDeviceLeftButtonHome`
  (params (Key :type "Key Structure" :default "AnyKey"))
  (bind _xdeviceplugin (`self.XDevicePlugin`))
  (:`Pressed`
    (set `self.LeftHomeButtonPressed` true)
    (if (`self.RightHomeButtonPressed`)
      (`XDevicePluginComponent.RecenterTracker` _xdeviceplugin :!label _label)
      (else
        (`XDevicePluginComponent.RecenterAllControllers` _xdeviceplugin :!label _label_2)))
    (`HeadMountedDisplayFunctionLibrary.ResetOrientationAndPosition` 0.0 "Orientation"))
  (:`Released`
    (set `self.LeftHomeButtonPressed` false)))

(event `Key|XDeviceRightButtonHome`
  (params (Key :type "Key Structure" :default "AnyKey"))
  (:`Pressed`
    (set `self.RightHomeButtonPressed` true)
    (if (`self.LeftHomeButtonPressed`)
      (goto _label)
      (else
        (goto _label_2))))
  (:`Released`
    (set `self.RightHomeButtonPressed` false)))

(event `Key|R`
  (params (Key :type "Key Structure" :default "AnyKey"))
  (:`Pressed`
    (goto _label_2)))

(event `Key|T`
  (params (Key :type "Key Structure" :default "AnyKey"))
  (:`Pressed`
    (goto _label)))

(fn `UserConstructionScript`)